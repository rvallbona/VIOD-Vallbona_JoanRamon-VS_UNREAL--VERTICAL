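; Door actor that slides in a straight line from its starting position to an end location when opened.
; BeginPlay stores the start location, and the OpenDoors event enables Tick.
; Tick accumulates time and lerps the actor location over the RotationRime duration, which drives translation despite its name, then disables itself.
; The file has no closing logic or timer reset.
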(event `self.ReceiveBeginPlay`
  ;[1 1 1] Logica de Abrir puerta
  ;;[1 1 1] Colocamos la puerta en la posicion inicial
  (set `self.StartLocation` (`self.K2_GetActorLocation`)))

(event `/Game/PuzzleInterface.OpenDoors`
  ;[1 1 1] Logica de Abrir puerta
  (`self.SetActorTickEnabled` true))

(event `self.ReceiveTick`
  (params (DeltaSeconds :type "Float (single-precision)"))
  ;[1 1 1] Logica de Abrir puerta
  ;;[1 1 1] Timer
  (set `self.CurrentTime` (+ DeltaSeconds (`self.CurrentTime`)))
  (`self.K2_SetActorLocation` (`KismetMathLibrary.VLerp` (`self.StartLocation`) (`self.EndLocation`) (/ (`self.CurrentTime`) (`self.RotationRime`))))
  (if (>= (`self.CurrentTime`) (`self.RotationRime`))
    (`self.SetActorTickEnabled` false)))

(fn `UserConstructionScript`)