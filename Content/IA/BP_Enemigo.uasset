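; BP_Enemigo is an enemy that chases pawns it sees and can be killed by damage.
; PawnSensing sightings drive an AI MoveTo toward the seen pawn, stopping within the enemy's acceptance radius.
; Any damage reduces Health, and falling below the minimum flags the enemy dead and destroys it.
; Health is copied into the HealthBar's WB_AIHealth widget only at BeginPlay, with no refresh after damage.
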(event `self.PawnSensing.OnSeePawn`
  (params (Pawn :type "Pawn Object Reference"))
  ;[1 1 1] Comprovacion de visión del Enemigo
  (`|AIMoveTo` self (0.0 0.0 0.0) Pawn (`self.EnemyRadius`)))

(event `self.ReceiveBeginPlay`
  ;[1 1 1] Updating Enemy Health Bar
  (`self.UpdateHealthBar`))

(event `self.ReceiveAnyDamage`
  (params (Damage :type "Float (single-precision)") (DamageType :type "DamageType Object Reference") (InstigatedBy :type "Controller Object Reference") (DamageCauser :type "Actor Object Reference"))
  ;[1 1 1] Updating Enemy Health Bar
  (set `self.Health` (- (`self.Health`) Damage))
  (if (< (`self.Health`) (`self.MinimHealth`))
    (set `self.isDead?` true)
    (`self.K2_DestroyActor`)))

(fn `UpdateHealthBar`
  (bind _aswb_aihealth (cast `/Game/IA/WB_AIHealth` (`WidgetComponent.GetUserWidgetObject` (`self.HealthBar`))))
  (set `/Game/IA/WB_AIHealth.Health` (`self.Health`) _aswb_aihealth)
  (return))

(fn `UserConstructionScript`)