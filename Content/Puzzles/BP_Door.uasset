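; BP_Door is a puzzle door actor that slides from its starting location to an end location when opened.
; BeginPlay caches the start location, and the OpenDoors event enables actor tick.
; Tick accumulates delta time and linearly interpolates the location over RotationRime, which acts as the move duration despite its name, then disables tick once that time has elapsed.
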(event `self.ReceiveBeginPlay`
  ;[1 1 1] OpenDoorLogic
  ;;[1 1 1] StartPositionDoor
  (set `self.StartLocation` (`self.K2_GetActorLocation`)))

(event `/Game/Puzzles/I_PuzzleInterface.OpenDoors`
  ;[1 1 1] OpenDoorLogic
  (`self.SetActorTickEnabled` true))

(event `self.ReceiveTick`
  (params (DeltaSeconds :type "Float (single-precision)"))
  ;[1 1 1] OpenDoorLogic
  ;;[1 1 1] Timer
  (set `self.CurrentTime` (+ DeltaSeconds (`self.CurrentTime`)))
  (`self.K2_SetActorLocation` (`KismetMathLibrary.VLerp` (`self.StartLocation`) (`self.EndLocation`) (/ (`self.CurrentTime`) (`self.RotationRime`))))
  (if (>= (`self.CurrentTime`) (`self.RotationRime`))
    (`self.SetActorTickEnabled` false)))

(fn `UserConstructionScript`)