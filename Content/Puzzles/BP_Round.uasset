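; BP_Round is a puzzle Blueprint that configures rotation data for three cube components.
; On BeginPlay it fills the Data array with one entry per cube, holding the component, its starting relative rotation and four single-axis rotation values in both directions.
; The graph only builds this data and contains no logic that applies the rotations.
; The construction script just calls its parent.
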(event `self.ReceiveBeginPlay`
  (bind _cube2 (`self.Cube2`))
  (bind _cube3 (`self.Cube3`))
  (bind _cube1 (`self.Cube1`))
  ;[1 1 1] Configuración de la "Data"
  (`KismetArrayLibrary.Array_Add` (`self.Data`) (make `/Game/Puzzles/S_BridgePuzzleData` _cube1 (`SceneComponent.RelativeRotation` _cube1) (`|MakeArray` (struct :`Yaw` 10.0) (struct :`Yaw` 25.0) (struct :`Yaw` -30.0) (struct :`Yaw` -15.0) :!type "Rotator Structure")))
  (`KismetArrayLibrary.Array_Add` (`self.Data`) (make `/Game/Puzzles/S_BridgePuzzleData` _cube2 (`SceneComponent.RelativeRotation` _cube2) (`|MakeArray` (struct :`Yaw` 40.0) (struct :`Yaw` 15.0) (struct :`Yaw` -10.0) (struct :`Yaw` -25.0) :!type "Rotator Structure")))
  (`KismetArrayLibrary.Array_Add` (`self.Data`) (make `/Game/Puzzles/S_BridgePuzzleData` _cube3 (`SceneComponent.RelativeRotation` _cube3) (`|MakeArray` (struct :`Yaw` 35.0) (struct :`Yaw` 25.0) (struct :`Yaw` -15.0) (struct :`Yaw` -5.0) :!type "Rotator Structure"))))

(fn `UserConstructionScript`
  (`parent.UserConstructionScript`))