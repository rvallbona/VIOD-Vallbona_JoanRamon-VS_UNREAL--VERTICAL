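; BP_FosaFuego is a fire pit hazard that sends the player to a respawn level on overlap.
; When a BP_FirstPersonCharacter enters, it disables movement and shows the WB_FadeChangeLevel widget.
; After the DurationTransition delay, it plays a 2D sound and opens RespawnLevel by name.
; A debug "Hello" print runs on every overlap, before the character cast.
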(event `self.ReceiveActorBeginOverlap`
  (params (OtherActor :type "Actor Object Reference"))
  (`KismetSystemLibrary.PrintText` "Hello")
  (bind _asbp_first_person_character (cast `/Game/FirstPerson/Blueprints/BP_FirstPersonCharacter` OtherActor))
  (set `/Game/FirstPerson/Blueprints/BP_FirstPersonCharacter.CanMove?` false _asbp_first_person_character)
  (`|ExecutionSequence`
    (:`then_0`
      (bind _returnvalue (`|CreateWidget` "/Game/UI/WB_FadeChangeLevel.WB_FadeChangeLevel_C"))
      (`UserWidget.AddToViewport` _returnvalue 0))
    (:`then_1`
      (`KismetSystemLibrary.Delay` (`self.durationTransition`))
      (`GameplayStatics.PlaySound2D` "/Engine/VREditor/Sounds/UI/Dockable_Window_Close.Dockable_Window_Close" 1.7 1.0 0.0 null null)
      (`GameplayStatics.OpenLevel` (`KismetStringLibrary.Conv_StringToName` (`self.RespawnLevel`))))))

(fn `UserConstructionScript`)